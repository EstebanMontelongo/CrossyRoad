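; Player chicken Blueprint that hops in fixed steps along the world X and Y axes from four directional input actions.
; Each press rotates the mesh toward the move, calls Jump and instantly offsets the actor's location, with IsJumping blocking further hops during a short Delay.
; Each hop also sets the camera to its own current world transform.
; Tick separately applies any consumed movement input, scaled by delta time, as a local offset to CharacterChicken.
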(event `InputAction|MoveLeft`
  (params (Key :type "Key Structure"))
  (bind (_returnvalue_x _returnvalue_y _returnvalue_z) (`KismetMathLibrary.BreakVector` (`self.K2_GetActorLocation`)))
  (bind _camera (`self.Camera`))
  (bind (_returnvalue_x_2 _returnvalue_y_2 _returnvalue_z_2) (`KismetMathLibrary.BreakVector` (`SceneComponent.K2_GetComponentLocation` _camera)))
  (:`Pressed`
    (if (not (`self.IsJumping`))
      (`SceneComponent.K2_SetRelativeRotation` (`self.Mesh`) (struct :`Yaw` 270.0) false false)
      (set `self.IsJumping` true)
      (`self.Jump`)
      (`self.K2_SetActorRelativeLocation` (`KismetMathLibrary.MakeVector` _returnvalue_x (+ _returnvalue_y -1000.0) _returnvalue_z))
      (`SceneComponent.K2_SetWorldLocationAndRotation` _camera (`KismetMathLibrary.MakeVector` _returnvalue_x_2 _returnvalue_y_2 _returnvalue_z_2) (`SceneComponent.K2_GetComponentRotation` _camera) false false)
      (`KismetSystemLibrary.Delay` 0.2)
      (set `self.IsJumping` false))))

(event `InputAction|MoveRight`
  (params (Key :type "Key Structure"))
  (bind (_returnvalue_x _returnvalue_y _returnvalue_z) (`KismetMathLibrary.BreakVector` (`self.K2_GetActorLocation`)))
  (bind _camera (`self.Camera`))
  (bind (_returnvalue_x_2 _returnvalue_y_2 _returnvalue_z_2) (`KismetMathLibrary.BreakVector` (`SceneComponent.K2_GetComponentLocation` _camera)))
  (:`Pressed`
    (if (not (`self.IsJumping`))
      (`SceneComponent.K2_SetRelativeRotation` (`self.Mesh`) (struct :`Yaw` -270.0) false false)
      (set `self.IsJumping` true)
      (`self.Jump`)
      (`self.K2_SetActorRelativeLocation` (`KismetMathLibrary.MakeVector` _returnvalue_x (+ 1000.0 _returnvalue_y) _returnvalue_z))
      (`SceneComponent.K2_SetWorldLocationAndRotation` _camera (`KismetMathLibrary.MakeVector` _returnvalue_x_2 _returnvalue_y_2 _returnvalue_z_2) (`SceneComponent.K2_GetComponentRotation` _camera) false false)
      (`KismetSystemLibrary.Delay` 0.2)
      (set `self.IsJumping` false))))

(event `self.ReceiveTick`
  (params (DeltaSeconds :type "Float (single-precision)"))
  (bind _returnvalue (`self.ConsumeMovementInputVector`))
  (`SceneComponent.K2_AddLocalOffset` (`self.character_chicken`) (* _returnvalue DeltaSeconds) false false))

(event `InputAction|MoveForward`
  (params (Key :type "Key Structure"))
  (bind (_returnvalue_x _returnvalue_y _returnvalue_z) (`KismetMathLibrary.BreakVector` (`self.K2_GetActorLocation`)))
  (bind _camera (`self.Camera`))
  (bind (_returnvalue_x_2 _returnvalue_y_2 _returnvalue_z_2) (`KismetMathLibrary.BreakVector` (`SceneComponent.K2_GetComponentLocation` _camera)))
  (:`Pressed`
    (if (not (`self.IsJumping`))
      (`SceneComponent.K2_SetRelativeRotation` :`self` (`self.Mesh`))
      (set `self.IsJumping` true)
      (`self.Jump`)
      (`self.K2_SetActorRelativeLocation` (`KismetMathLibrary.MakeVector` (+ 1000.0 _returnvalue_x) _returnvalue_y _returnvalue_z))
      (`SceneComponent.K2_SetWorldLocationAndRotation` _camera (`KismetMathLibrary.MakeVector` _returnvalue_x_2 _returnvalue_y_2 _returnvalue_z_2) (`SceneComponent.K2_GetComponentRotation` _camera) false false)
      (`KismetSystemLibrary.Delay` 0.2)
      (set `self.IsJumping` false))))

(event `InputAction|MoveBack`
  (params (Key :type "Key Structure"))
  (bind (_returnvalue_x _returnvalue_y _returnvalue_z) (`KismetMathLibrary.BreakVector` (`self.K2_GetActorLocation`)))
  (bind _camera (`self.Camera`))
  (bind (_returnvalue_x_2 _returnvalue_y_2 _returnvalue_z_2) (`KismetMathLibrary.BreakVector` (`SceneComponent.K2_GetComponentLocation` _camera)))
  (:`Pressed`
    (if (not (`self.IsJumping`))
      (`SceneComponent.K2_SetRelativeRotation` (`self.Mesh`) (struct :`Yaw` 180.0) false false)
      (set `self.IsJumping` true)
      (`self.Jump`)
      (`self.K2_SetActorRelativeLocation` (`KismetMathLibrary.MakeVector` (+ -1000.0 _returnvalue_x) _returnvalue_y _returnvalue_z))
      (`SceneComponent.K2_SetWorldLocationAndRotation` _camera (`KismetMathLibrary.MakeVector` _returnvalue_x_2 _returnvalue_y_2 _returnvalue_z_2) (`SceneComponent.K2_GetComponentRotation` _camera) false false)
      (`KismetSystemLibrary.Delay` 0.2)
      (set `self.IsJumping` false))))

(fn `UserConstructionScript`)