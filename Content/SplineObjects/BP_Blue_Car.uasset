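; BP_Blue_Car is a car actor that drives along the spline of a referenced track actor.
; When flagged active on BeginPlay, it plays a timeline whose rate is set by Duration and whose start time comes from CarStartOffset.
; Each update maps the timeline alpha to a distance along the spline and sets the car's world location and rotation.
; A ReturnBlueCar function returns the actor itself.
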(event `self.ReceiveBeginPlay`
  (if (`self.ActiveCar`)
    (`self.MoveCar`)))

(event `MoveCar`
  (bind _returnvalue (`KismetMathLibrary.Lerp` 0.0 (`SplineComponent.GetSplineLength` (`/Game/SplineObjects/BP_Track.SplineTest` (`self.TrackRef`))) (`self.Alpha`)))
  (`TimelineComponent.SetPlayRate` (`self.CarMover`) (/ 1.0 (`self.Duration`)))
  (`TimelineComponent.SetNewTime` (`self.CarMover`) (`self.CarStartOffset`))
  (bind (_direction _alpha) (`Timeline|CarMover`)
    (:`Update`
      (set `self.Alpha` _alpha)
      (`self.K2_SetActorLocationAndRotation` (`SplineComponent.GetLocationAtDistanceAlongSpline` (`/Game/SplineObjects/BP_Track.SplineTest` (`self.TrackRef`)) _returnvalue "World") (`SplineComponent.GetRotationAtDistanceAlongSpline` (`/Game/SplineObjects/BP_Track.SplineTest` (`self.TrackRef`)) _returnvalue "World")))))

(fn `ReturnBlueCar`
  (returns (NewParam :type "/Game/SplineObjects/BP_Blue_Car Object Reference"))
  (return self))

(fn `UserConstructionScript`)